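; BP_Tunnel is one segment of an endless tunnel: crossing its trigger adds score, asks TunnelSpawner for another segment and destroys this one.
; Its rotating wall and star enemy damage the player, triggering restart at zero health, while health packs heal.
; Projectiles destroy enemies for score and camera shake, and overlaps refresh HUD displays.
; Randomize functions vary wall mesh and roll, enemy position, and health pack presence and position.
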(event OnComponentBeginOverlap(TriggerZone)
  (params (OverlappedComponent :type Primitive%20Component%20Object%20Reference) (OtherActor :type Actor%20Object%20Reference) (OtherComp :type Primitive%20Component%20Object%20Reference) (OtherBodyIndex :type Integer) (bFromSweep :type Boolean) (SweepResult :type Hit%20Result%20Structure%20%28by%20ref%29))
  (Utilities|FlowControl|Sequence
    (:then_0
      (bind _asbp_player (Utilities|Casting|CastToBP_Player OtherActor))
      (Variables|/Game/InfiniteMatrix/Blueprints/BP_Player.BP_Player_C|SetScore _asbp_player (+ (Variables|/Game/InfiniteMatrix/Blueprints/BP_Player.BP_Player_C|GetScore _asbp_player) 1.0)))
    (:then_1
      (bind _asnew_hud (Utilities|Casting|CastToNewHUD (HUD|GetHUD (Game|GetPlayerController 0))))
      (Default|UpdateScore (Variables|/Game/Blueprints/NewHUD.NewHUD_C|GetScoreDisplay _asnew_hud)))
    (:then_2
      (Utilities|Casting|CastToBP_Player OtherActor)
      (Default|SpawnTunnelatSpawnPoint (Variables|Default|GetTunnelSpawner))
      (Actor|DestroyActor))))

(event OnComponentBeginOverlap(HealthPackMesh)
  (params (OverlappedComponent :type Primitive%20Component%20Object%20Reference) (OtherActor :type Actor%20Object%20Reference) (OtherComp :type Primitive%20Component%20Object%20Reference) (OtherBodyIndex :type Integer) (bFromSweep :type Boolean) (SweepResult :type Hit%20Result%20Structure%20%28by%20ref%29))
  (Utilities|FlowControl|Sequence
    (:then_0
      (bind _asbp_player (Utilities|Casting|CastToBP_Player OtherActor))
      (if (not (>= (Variables|/Game/InfiniteMatrix/Blueprints/BP_Player.BP_Player_C|GetHealth _asbp_player) 1e+02))
        (Variables|/Game/InfiniteMatrix/Blueprints/BP_Player.BP_Player_C|SetHealth _asbp_player (+ (Variables|/Game/InfiniteMatrix/Blueprints/BP_Player.BP_Player_C|GetHealth _asbp_player) 1e+01))))
    (:then_1
      (bind _asnew_hud (Utilities|Casting|CastToNewHUD (HUD|GetHUD (Game|GetPlayerController 0))))
      (Default|UpdateText (Variables|/Game/Blueprints/NewHUD.NewHUD_C|GetHealthDisplay _asnew_hud)))
    (:then_2
      (Utilities|Casting|CastToBP_Player OtherActor)
      (Components|DestroyComponent OverlappedComponent))))

(event OnComponentBeginOverlap(WallMesh)
  (params (OverlappedComponent :type Primitive%20Component%20Object%20Reference) (OtherActor :type Actor%20Object%20Reference) (OtherComp :type Primitive%20Component%20Object%20Reference) (OtherBodyIndex :type Integer) (bFromSweep :type Boolean) (SweepResult :type Hit%20Result%20Structure%20%28by%20ref%29))
  (Utilities|FlowControl|Sequence
    (:then_0
      (bind _asbp_player (Utilities|Casting|CastToBP_Player OtherActor))
      (Variables|/Game/InfiniteMatrix/Blueprints/BP_Player.BP_Player_C|SetHealth _asbp_player (- (Variables|/Game/InfiniteMatrix/Blueprints/BP_Player.BP_Player_C|GetHealth _asbp_player) 1e+01)))
    (:then_1
      (bind _asbp_player_2 (Utilities|Casting|CastToBP_Player OtherActor))
      (if (<= (Variables|/Game/InfiniteMatrix/Blueprints/BP_Player.BP_Player_C|GetHealth _asbp_player_2) 0.0)
        (Variables|/Game/InfiniteMatrix/Blueprints/BP_Player.BP_Player_C|SetIsDead _asbp_player_2 true)
        (Default|DisplayRestart _asbp_player_2)))
    (:then_2
      (bind _asbp_player_3 (Utilities|Casting|CastToBP_Player OtherActor))
      (Variables|/Game/InfiniteMatrix/Blueprints/BP_Player.BP_Player_C|SetScore _asbp_player_3 (- (Variables|/Game/InfiniteMatrix/Blueprints/BP_Player.BP_Player_C|GetScore _asbp_player_3) 1.0)))
    (:then_3
      (bind _asnew_hud (Utilities|Casting|CastToNewHUD (HUD|GetHUD (Game|GetPlayerController 0))))
      (Default|UpdateText (Variables|/Game/Blueprints/NewHUD.NewHUD_C|GetHealthDisplay _asnew_hud)))))

(event OnComponentBeginOverlap(EnemyMesh)
  (params (OverlappedComponent :type Primitive%20Component%20Object%20Reference) (OtherActor :type Actor%20Object%20Reference) (OtherComp :type Primitive%20Component%20Object%20Reference) (OtherBodyIndex :type Integer) (bFromSweep :type Boolean) (SweepResult :type Hit%20Result%20Structure%20%28by%20ref%29))
  (Utilities|FlowControl|Sequence
    (:then_0
      (bind _asbp_player (Utilities|Casting|CastToBP_Player OtherActor))
      (Variables|/Game/InfiniteMatrix/Blueprints/BP_Player.BP_Player_C|SetHealth _asbp_player (- (Variables|/Game/InfiniteMatrix/Blueprints/BP_Player.BP_Player_C|GetHealth _asbp_player) 1e+01))
      (Components|DestroyComponent OverlappedComponent)
      (bind _asnew_hud (Utilities|Casting|CastToNewHUD (HUD|GetHUD (Game|GetPlayerController 0))))
      (Default|UpdateText (Variables|/Game/Blueprints/NewHUD.NewHUD_C|GetHealthDisplay _asnew_hud)))
    (:then_1
      (bind _asbp_player_2 (Utilities|Casting|CastToBP_Player OtherActor)
        (:then
          (if (<= (Variables|/Game/InfiniteMatrix/Blueprints/BP_Player.BP_Player_C|GetHealth _asbp_player_2) 0.0)
            (Variables|/Game/InfiniteMatrix/Blueprints/BP_Player.BP_Player_C|SetIsDead _asbp_player_2 true)
            (Default|DisplayRestart _asbp_player_2)))
        (:CastFailed
          (Utilities|Casting|CastToBP_Projectile OtherActor)
          (bind _asbp_player_3 (Utilities|Casting|CastToBP_Player (Game|Player|GetPlayerPawn 0)))
          (Variables|/Game/InfiniteMatrix/Blueprints/BP_Player.BP_Player_C|SetScore _asbp_player_3 (+ (Variables|/Game/InfiniteMatrix/Blueprints/BP_Player.BP_Player_C|GetScore _asbp_player_3) 1.0))
          (Components|DestroyComponent OverlappedComponent)
          (bind _asnew_hud_2 (Utilities|Casting|CastToNewHUD (HUD|GetHUD (Game|GetPlayerController 0))))
          (Default|UpdateScore (Variables|/Game/Blueprints/NewHUD.NewHUD_C|GetScoreDisplay _asnew_hud_2))
          (Camera|PlayWorldCameraShake "/Game/InfiniteMatrix/Blueprints/Shake.Shake_C" (Transformation|GetActorLocation _asbp_player_3) 0.0 5e+02))))))

(event EventBeginPlay)

(event EventTick
  (params (DeltaSeconds :type Float%20%28single-precision%29))
  (Transformation|AddLocalRotation (Variables|Default|GetWallMesh) (Math|Rotator|MakeRotator (* DeltaSeconds (Variables|Default|GetRotateSpeed)) 0.0 0.0) false false))

(fn ConstructionScript)

(fn RandomizeWall
  (Components|StaticMesh|SetStaticMesh (Variables|Default|GetWallMesh) (Utilities|Select :Index (Math|Random|RandomIntegerinRange 0 3) :Option%200 "/Game/InfiniteMatrix/Meshes/SM_Hole_01.SM_Hole_01" :Option%201 "/Game/InfiniteMatrix/Meshes/SM_Hole_02.SM_Hole_02" :Option%202 "/Game/InfiniteMatrix/Meshes/SM_Hole_03.SM_Hole_03" :Option%203 "/Game/InfiniteMatrix/Meshes/SM_Hole_04.SM_Hole_04"))
  (Transformation|AddLocalRotation (Variables|Default|GetWallMesh) (Math|Rotator|MakeRotator (Math|Random|RandomFloatinRange 0.0 3.6e+02) 0.0 0.0) false false))

(fn RandomizeHealthPack
  (Components|StaticMesh|SetStaticMesh (Variables|Default|GetHealthPackMesh) (Utilities|Select :Index (Math|Random|RandomIntegerinRange 0 3) :Option%200 "/Game/InfiniteMatrix/Meshes/SM_HealthPack.SM_HealthPack" :Option%201 0 :Option%202 0 :Option%203 0))
  (Transformation|AddLocalOffset (Variables|Default|GetHealthPackMesh) (Math|Vector|MakeVector (Math|Conversions|ToFloat(Integer) (Math|Random|RandomIntegerinRange -60 60)) (Math|Conversions|ToFloat(Integer) (Math|Random|RandomIntegerinRange 100 2370)) (Math|Conversions|ToFloat(Integer) (Math|Random|RandomIntegerinRange -60 60))) false false))

(fn RandomizeEnemy
  (Components|StaticMesh|SetStaticMesh (Variables|Default|GetEnemyMesh) "/Game/InfiniteMatrix/Meshes/Star.Star")
  (Transformation|AddLocalOffset (Variables|Default|GetEnemyMesh) (Math|Vector|MakeVector (Math|Random|RandomFloatinRange -1.2e+02 1.2e+02) (Math|Random|RandomFloatinRange 1e+02 2.37e+03) (Math|Random|RandomFloatinRange -1.2e+02 1.2e+02)) false false)
  (Class|PrimitiveComponent|SetEmissiveLightSource (Variables|Default|GetEnemyMesh) true))